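; Player actor Blueprint for a mouse-controlled game in which overlapping any actor ends the round.
; Mouse axis input offsets the actor along world X and Y without sweeping while CanMove is true.
; An overlap sets GameOver on gm_BP and freezes movement, after which a left click triggers Restart.
; Restart, also run on BeginPlay, clears the game mode's GameOver and GameWon flags, returns to SpawnLocation and re-enables movement.
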(event `Restart`
  (bind _asgm_bp (cast `/Game/res/gm_BP` (`GameplayStatics.GetGameMode`) :!label _label))
  (set `/Game/res/gm_BP.GameOver` false _asgm_bp)
  (set `/Game/res/gm_BP.GameWon` false _asgm_bp)
  (`self.K2_SetActorTransform` (`self.SpawnLocation`))
  (set `self.CanMove` true))

(event `self.ReceiveBeginPlay`
  (goto _label))

(event `InputAxis|MouseX`
  (params (AxisValue :type "Float (single-precision)"))
  (if (`self.CanMove`)
    (`self.K2_AddActorWorldOffset` (`KismetMathLibrary.MakeVector` AxisValue 0.0 0.0))))

(event `InputAxis|MouseY`
  (params (AxisValue :type "Float (single-precision)"))
  (if (`self.CanMove`)
    (`self.K2_AddActorWorldOffset` (`KismetMathLibrary.MakeVector` 0.0 AxisValue))))

(event `self.ReceiveActorBeginOverlap`
  (params (OtherActor :type "Actor Object Reference"))
  (bind _asgm_bp (cast `/Game/res/gm_BP` (`GameplayStatics.GetGameMode`)))
  (set `/Game/res/gm_BP.GameOver` true _asgm_bp)
  (set `self.CanMove` false))

(event `InputAction|MouseLeftClick`
  (params (Key :type "Key Structure"))
  (:`Pressed`
    (if (not (`self.CanMove`))
      (`self.Restart`))))

(fn `UserConstructionScript`)